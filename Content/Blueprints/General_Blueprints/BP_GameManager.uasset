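; BP_GameManager loads and saves persistent player data, tracking a play count.
; On BeginPlay it creates a default BP_SavePlayerData to supply the slot name and user index, replaces it with any loaded save, and prints PlayNumber.
; On EndPlay, only when IsOpeningLevel is true, it increments PlayNumber and writes the save to that slot.
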(event EventBeginPlay
  (CallFunction|LoadPlayerData))

(event EventTick
  (params (DeltaSeconds :type Float%20%28single-precision%29)))

(event EventEndPlay
  (params (EndPlayReason :type EEndPlayReason%20Enum :default "Destroyed"))
  (CallFunction|SavePlayerData))

(fn ConstructionScript)

(fn LoadPlayerData
  (bind _returnvalue (SaveGame|CreateSaveGameObject "/Game/Blueprints/General_Blueprints/BP_SavePlayerData.BP_SavePlayerData_C"))
  (bind _output_get (Variables|Default|SetPlayerDataInstance _returnvalue))
  (bind _returnvalue_2 (SaveGame|LoadGamefromSlot (Variables|/Game/Blueprints/General_Blueprints/BP_SavePlayerData.BP_SavePlayerData_C|GetSaveSlotName _output_get) (Variables|/Game/Blueprints/General_Blueprints/BP_SavePlayerData.BP_SavePlayerData_C|GetUserIndex _output_get)))
  (bind _asbp_save_player_data (Utilities|Casting|CastToBP_SavePlayerData _returnvalue_2))
  (bind _output_get_2 (Variables|Default|SetPlayerDataInstance _asbp_save_player_data))
  (Development|PrintString (Utilities|String|ToString(Integer) (Variables|/Game/Blueprints/General_Blueprints/BP_SavePlayerData.BP_SavePlayerData_C|GetPlayNumber _output_get_2))))

(fn SavePlayerData
  (bind _playerdatainstance (Variables|Default|GetPlayerDataInstance))
  (if (Variables|Default|GetIsOpeningLevel)
    (Math|Integer|IncrementInt (Variables|/Game/Blueprints/General_Blueprints/BP_SavePlayerData.BP_SavePlayerData_C|GetPlayNumber _playerdatainstance)
      (:%20%20
        (SaveGame|SaveGametoSlot _playerdatainstance (Variables|/Game/Blueprints/General_Blueprints/BP_SavePlayerData.BP_SavePlayerData_C|GetSaveSlotName _playerdatainstance) (Variables|/Game/Blueprints/General_Blueprints/BP_SavePlayerData.BP_SavePlayerData_C|GetUserIndex _playerdatainstance))))))