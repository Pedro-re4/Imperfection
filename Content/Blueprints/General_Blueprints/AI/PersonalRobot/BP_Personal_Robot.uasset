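; Personal robot AI character that caches its navigation context and reports target point overlaps to its AI blackboard.
; On BeginPlay it stores interaction point world locations in an array, applies its walk speed and caches the first-person player found by class.
; Overlapping a BP_TargetPoint calls ResetDialogueVar, which sets the controller blackboard's IsOverlapping flag to true.
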(event EventBeginPlay
  (|CallParentFunction)
  (CallFunction|SetInteractionPointsLoc)
  (Variables|/Script/Engine.CharacterMovementComponent|SetMaxWalkSpeed (Variables|Character|GetCharacterMovement) (Variables|Default|GetWalkSpeed))
  (bind _outactors (Actor|GetAllActorsOfClass "/Game/Blueprints/Player_Controller/BP_First_Person_Character.BP_First_Person_Character_C"))
  (Variables|Default|SetPlayer (Utilities|Array|Get(acopy) _outactors)))

(event Collision|EventActorBeginOverlap
  (params (OtherActor :type Actor%20Object%20Reference))
  (if (== (Utilities|GetClass OtherActor) "/Game/Blueprints/General_Blueprints/BP_TargetPoint.BP_TargetPoint_C")
    (CallFunction|ResetDialogueVar true)))

(event EventTick
  (params (DeltaSeconds :type Float%20%28single-precision%29))
  (|CallParentFunction DeltaSeconds) ; This node is disabled and will not be called.\nDrag off pins to build functionality.
)

(fn ConstructionScript
  (|CallParentFunction))

(fn SetInteractionPointsLoc
  (for (_array_element _array_index) (Variables|Default|GetInteractionPoints)
    (Utilities|Array|SetArrayElem (Variables|Default|GetInteractionPointsLocation) _array_index (Transformation|GetWorldLocation (Variables|/Script/Engine.Actor|GetRootComponent _array_element)) true)))

(fn ResetDialogueVar
  (params (VarValue :type Boolean))
  (AI|Components|Blackboard|SetValueasBool (AI|GetBlackboard (Pawn|GetController)) (Variables|Default|GetIsOverlapping) VarValue))